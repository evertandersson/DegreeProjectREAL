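; Gameplay ability that makes the third-person character perform a dodge roll.
; On activation it commits, disables jumping and snaps the character toward its last movement input, if any.
; It then plays the roll montage alongside a constant root motion force along the actor's forward vector, ending when that force finishes.
; Ending the ability re-enables jumping and removes the loose combo window tags.
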(event `self.K2_ActivateAbility`
  (bind _returnvalue (`self.GetAvatarActorFromActorInfo`))
  (`self.K2_CommitAbility`)
  (`self.SetRotation`)
  (`AbilityTask_PlayMontageAndWait.CreatePlayMontageAndWaitProxy` "None" "/Game/Characters/Player/Animations/NewAnimations/AM_Roll.AM_Roll"
    (:`then`
      (`AbilityTask_ApplyRootMotionConstantForce.ApplyRootMotionConstantForce` "None" (`Actor.GetActorForwardVector` _returnvalue) 1000.0 0.8 false null "ClampVelocity" (`Actor.GetVelocity` _returnvalue)
        (:`OnFinish`
          (`self.K2_EndAbility`))))))

(event `self.K2_OnEndAbility`
  (params (bWasCancelled :type Boolean))
  (set `DegreeProjectCharacter.bCanJump` true (`self.ThirdPersonCharacter`))
  (`AbilitySystemBlueprintLibrary.RemoveLooseGameplayTags` (`self.GetAvatarActorFromActorInfo`) (`self.Combo Window`))
  (`AbilitySystemBlueprintLibrary.RemoveLooseGameplayTags` (`self.GetAvatarActorFromActorInfo`) (`self.Combo Window 2`)))

(fn `SetRotation`
  (bind _asbp_third_person_character (cast `/Game/ThirdPerson/Blueprints/BP_ThirdPersonCharacter` (`self.GetAvatarActorFromActorInfo`)))
  (set `self.ThirdPersonCharacter` _asbp_third_person_character)
  (set `DegreeProjectCharacter.bCanJump` false _asbp_third_person_character)
  (bind _returnvalue (`PawnMovementComponent.GetLastInputVector` (`Character.CharacterMovement` _asbp_third_person_character)))
  (if (`KismetMathLibrary.NotEqualExactly_VectorVector` _returnvalue)
    (`Actor.K2_SetActorRotation` _asbp_third_person_character (`KismetMathLibrary.MakeRotFromX` _returnvalue) false)))