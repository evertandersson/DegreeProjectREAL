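; GA_Stagger is a Gameplay Ability that staggers the third-person player character, locking its movement while a reaction montage plays.
; On activation it commits, resolves the avatar as BP_ThirdPersonCharacter when no valid reference is stored, and sets movement mode to None.
; It then plays AM_Stagger, and any montage outcome (completed, blend out, interrupted or cancelled) restores Walking and ends the ability.
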(event `self.K2_ActivateAbility`
  (`self.K2_CommitAbility`)
  (`/Engine/EditorBlueprintResources/StandardMacros.IsValid` (`self.PlayerRef`)
    (:`Is Valid`
      _)
    (:`Is Not Valid`
      (bind _asbp_third_person_character (cast `/Game/ThirdPerson/Blueprints/BP_ThirdPersonCharacter` (`self.GetAvatarActorFromActorInfo`)))))
  (bind _output_get (set `self.PlayerRef` _asbp_third_person_character))
  (bind _charactermovement (`Character.CharacterMovement` _output_get))
  (`CharacterMovementComponent.SetMovementMode` _charactermovement "MOVE_None" 0)
  (`AbilityTask_PlayMontageAndWait.CreatePlayMontageAndWaitProxy` "None" "/Game/Characters/Player/Animations/NewAnimations/AM_Stagger.AM_Stagger" 1.0 "None" true 1.0 0.0 true
    (:`OnCompleted`
      _)
    (:`OnBlendOut`
      _)
    (:`OnInterrupted`
      _)
    (:`OnCancelled`
      _))
  (`CharacterMovementComponent.SetMovementMode` _charactermovement "MOVE_Walking" 0)
  (`self.K2_EndAbility`))