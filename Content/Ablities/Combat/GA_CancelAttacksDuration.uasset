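; GA_CancelAttacksDuration is a player Gameplay Ability that clears combo and grapple state, then stays active until a clearing ability activates.
; On activation it commits and strips both combo window loose tags from the avatar without replication.
; It resets the third-person character's grapple hook if that character is grappling or rotating toward a grapple point.
; It then waits for an ability tagged Player.CancelClearAttacks to activate and ends itself.
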(event `self.K2_ActivateAbility`
  (bind _returnvalue (`self.GetAvatarActorFromActorInfo`))
  (`self.K2_CommitAbility`)
  (`AbilitySystemBlueprintLibrary.RemoveLooseGameplayTags` (`self.GetAvatarActorFromActorInfo`) (`self.Combo Window`))
  (`AbilitySystemBlueprintLibrary.RemoveLooseGameplayTags` _returnvalue (`self.Combo Window 2`))
  (bind _asbp_third_person_character (cast `/Game/ThirdPerson/Blueprints/BP_ThirdPersonCharacter` _returnvalue))
  (bind _grapplingcomponent (`DegreeProjectCharacter.GrapplingComponent` _asbp_third_person_character))
  (if (or (`GrapplingComponent.bIsRotatingTowardsGrapplePoint` _grapplingcomponent) (`GrapplingComponent.bIsGrappling` _grapplingcomponent))
    (`/Game/ThirdPerson/Blueprints/BP_ThirdPersonCharacter.Reset Grapple Hook` _asbp_third_person_character false))
  (`AbilityTask_WaitAbilityActivate.WaitForAbilityActivate` (struct :`TagName` "Player.CancelClearAttacks")
    (:`OnActivate`
      (`self.K2_EndAbility`))))

(event `self.K2_OnEndAbility`
  (params (bWasCancelled :type Boolean)))