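; Gameplay ability for a combat attack that can land a critical hit on the avatar's enemy.
; On activation it commits, then compares a stepped random percentage roll against an ability-system attribute.
; A successful roll applies damage as the product of two attributes; otherwise it applies a single attribute's value.
; The target comes from an enemy-reference interface message, which is called only on the crit branch though both branches use its result.
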(event `self.K2_ActivateAbility`
  (bind _returnvalue (`self.GetAvatarActorFromActorInfo`))
  (bind _returnvalue_2 (`Actor.GetOwner` _returnvalue))
  (bind _returnvalue_3 (`AbilitySystemBlueprintLibrary.GetAbilitySystemComponent` _returnvalue))
  (bind (_bsuccessfullyfoundattribute _returnvalue_4) (`AbilitySystemBlueprintLibrary.GetFloatAttributeFromAbilitySystemComponent` _returnvalue_3 (struct :`AttributeName` "Damage" :`Attribute` "/Script/DegreeProject.StandardAttributeSet:Damage" :`AttributeOwner` "/Script/CoreUObject.Class'/Script/DegreeProject.StandardAttributeSet'")))
  (`self.K2_CommitAbility`)
  (set `self.RandomInt` (- (* (`KismetMathLibrary.RandomIntegerInRange` 1 10) 10) 1))
  (if (< (`self.RandomInt`) (`.ReturnValue` (`AbilitySystemBlueprintLibrary.GetFloatAttributeFromAbilitySystemComponent` (`AbilitySystemBlueprintLibrary.GetAbilitySystemComponent` (`self.GetAvatarActorFromActorInfo`)) (struct :`AttributeName` "Crit_Chance" :`Attribute` "/Script/DegreeProject.StandardAttributeSet:Crit_Chance" :`AttributeOwner` "/Script/CoreUObject.Class'/Script/DegreeProject.StandardAttributeSet'"))))
    (bind _enemyref (message `/Game/ThirdPerson/Blueprints/Interfaces/I_Enemy.GetEnemyRef` _returnvalue))
    (`GameplayStatics.ApplyDamage` _enemyref (* _returnvalue_4 (`.ReturnValue` (`AbilitySystemBlueprintLibrary.GetFloatAttributeFromAbilitySystemComponent` _returnvalue_3 (struct :`AttributeName` "Crit_Damage" :`Attribute` "/Script/DegreeProject.StandardAttributeSet:Crit_Damage" :`AttributeOwner` "/Script/CoreUObject.Class'/Script/DegreeProject.StandardAttributeSet'")))) null _returnvalue_2)
    (else
      (`GameplayStatics.ApplyDamage` _enemyref _returnvalue_4 null _returnvalue_2))))