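; GA_Combo1 is a Gameplay Ability for a combo attack, apparently the first step, that plays a montage and manages a combo window.
; On activation it commits, starts the montage and listens for CombatWindowOpen and CombatWindowEnd gameplay events in parallel.
; Open adds a non-replicated loose combo-window tag to the avatar; End removes it and ends the ability.
; Montage completion also ends the ability, without removing the tag.
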(event `self.K2_ActivateAbility`
  (`self.K2_CommitAbility`)
  (`AbilityTask_PlayMontageAndWait.CreatePlayMontageAndWaitProxy` "None" (`self.Montage to Play`)
    (:`then`
      (`AbilityTask_WaitGameplayEvent.WaitGameplayEvent` (struct :`TagName` "Event.CombatWindowOpen") null
        (:`then`
          (`AbilityTask_WaitGameplayEvent.WaitGameplayEvent` (struct :`TagName` "Event.CombatWindowEnd") null
            (:`EventReceived`
              (`KismetSystemLibrary.PrintString` "Combo1 WindowClosed")
              (`AbilitySystemBlueprintLibrary.RemoveLooseGameplayTags` (`self.GetAvatarActorFromActorInfo`) (`self.ComboWindowOpenTag`))
              (`self.K2_EndAbility`))))
        (:`EventReceived`
          (`KismetSystemLibrary.PrintString` "Combo1 WindowOpen")
          (`AbilitySystemBlueprintLibrary.AddLooseGameplayTags` (`self.GetAvatarActorFromActorInfo`) (`self.ComboWindowOpenTag`)))))
    (:`OnCompleted`
      (`self.K2_EndAbility`))))

(event `self.K2_OnEndAbility`
  (params (bWasCancelled :type Boolean))
  (`KismetSystemLibrary.PrintString` "Combo1 Ended"))