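; Gameplay ability for the third step of the spear combo, playing its attack montage from partway in.
; On activation it commits, clears the owner's list of hit enemies and disables jumping and climbing through messages to the owner.
; A combat-window-end gameplay event removes the combo-window-open loose tag from the avatar.
; Montage completion ends the ability, and ending restores jumping and climbing.
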(event `self.K2_ActivateAbility`
  (bind _returnvalue (`self.GetOwningActorFromActorInfo`))
  (`self.K2_CommitAbility`)
  (message `/Game/ThirdPerson/Blueprints/Interfaces/I_GASOwner.ClearEnemiesHit` _returnvalue)
  (message `IHasGroundPos.ToggleCanJump` _returnvalue false)
  (message `IHasGroundPos.ToggleCanClimb` _returnvalue false)
  (`AbilityTask_PlayMontageAndWait.CreatePlayMontageAndWaitProxy` "None" (`self.MontageToPlay`) 1.0 "None" true 1.0 0.6
    (:`then`
      (`AbilityTask_WaitGameplayEvent.WaitGameplayEvent` (struct :`TagName` "Event.CombatWindowEnd") null
        (:`EventReceived`
          (`KismetSystemLibrary.PrintString` "Combo3 WindowClosed")
          (`AbilitySystemBlueprintLibrary.RemoveLooseGameplayTags` (`self.GetAvatarActorFromActorInfo`) (`self.ComboWindowOpenTag`)))))
    (:`OnCompleted`
      (`self.K2_EndAbility`))))

(event `self.K2_OnEndAbility`
  (params (bWasCancelled :type Boolean))
  (bind _returnvalue (`self.GetOwningActorFromActorInfo`))
  (`KismetSystemLibrary.PrintString` "Combo3 Ended")
  (message `IHasGroundPos.ToggleCanJump` _returnvalue true)
  (message `IHasGroundPos.ToggleCanClimb` _returnvalue true))