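; GA_Combo3 is a gameplay ability for the third step of a combat combo.
; On activation it commits, plays a montage and, alongside it, waits for the Event.CombatWindowEnd gameplay event.
; That event removes the loose combo-window-open tag from the avatar without replication, while montage completion ends the ability.
; Debug strings print when the window closes and the ability ends.
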(event `self.K2_ActivateAbility`
  (`self.K2_CommitAbility`)
  (`AbilityTask_PlayMontageAndWait.CreatePlayMontageAndWaitProxy` "None" (`self.Montage to Play`)
    (:`then`
      (`AbilityTask_WaitGameplayEvent.WaitGameplayEvent` (struct :`TagName` "Event.CombatWindowEnd") null
        (:`EventReceived`
          (`KismetSystemLibrary.PrintString` "Combo3 WindowClosed")
          (`AbilitySystemBlueprintLibrary.RemoveLooseGameplayTags` (`self.GetAvatarActorFromActorInfo`) (`self.ComboWindowOpenTag`)))))
    (:`OnCompleted`
      (`self.K2_EndAbility`))))

(event `self.K2_OnEndAbility`
  (params (bWasCancelled :type Boolean))
  (`KismetSystemLibrary.PrintString` "Combo3 Ended"))