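; GA_Combo1 is a Gameplay Ability that plays a sword combo attack montage and manages its combo window.
; On activation it commits, clears the owner's hit-enemy record and disables jumping, which is restored when the ability ends.
; Combat window gameplay events add and remove a loose, non-replicated combo-window tag on the avatar.
; The ability ends when the window closes or the montage completes.
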(event `self.K2_ActivateAbility`
  (bind _returnvalue (`self.GetOwningActorFromActorInfo`))
  (`self.K2_CommitAbility`)
  (message `/Game/ThirdPerson/Blueprints/Interfaces/I_GASOwner.ClearEnemiesHit` _returnvalue)
  (message `IHasGroundPos.ToggleCanJump` _returnvalue false)
  (`AbilityTask_PlayMontageAndWait.CreatePlayMontageAndWaitProxy` "None" (`self.MontageToPlay`)
    (:`then`
      (`AbilityTask_WaitGameplayEvent.WaitGameplayEvent` (struct :`TagName` "Event.CombatWindowOpen") null
        (:`then`
          (`AbilityTask_WaitGameplayEvent.WaitGameplayEvent` (struct :`TagName` "Event.CombatWindowEnd") null
            (:`EventReceived`
              (`KismetSystemLibrary.PrintString` "Combo1 WindowClosed")
              (`AbilitySystemBlueprintLibrary.RemoveLooseGameplayTags` (`self.GetAvatarActorFromActorInfo`) (`self.ComboWindowOpenTag`))
              (`self.K2_EndAbility`))))
        (:`EventReceived`
          (`KismetSystemLibrary.PrintString` "Combo1 WindowOpen")
          (`AbilitySystemBlueprintLibrary.AddLooseGameplayTags` (`self.GetAvatarActorFromActorInfo`) (`self.ComboWindowOpenTag`)))))
    (:`OnCompleted`
      (`self.K2_EndAbility`))))

(event `self.K2_OnEndAbility`
  (params (bWasCancelled :type Boolean))
  (`KismetSystemLibrary.PrintString` "Combo1 Ended")
  (message `IHasGroundPos.ToggleCanJump` (`self.GetOwningActorFromActorInfo`) true))