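; Enemy spawner Blueprint that handles round-based feedback: remaining-enemy highlighting, boss music and end-of-round skill display.
; Tick derives enemies left from spawn and kill counts, toggling custom depth on all enemy meshes when three or fewer remain.
; Tick also checks round indices to play the boss theme once and stop it when rounds finish.
; Game manager new-round events call OnNewRoundBegin, while RoundEnded calls DisplaySkills.
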(event `self.ReceiveTick`
  (params (DeltaSeconds :type "Float (single-precision)"))
  (`|ExecutionSequence`
    (:`then_0`
      (`self.Remaining enemies event`))
    (:`then_1`
      (`self.Get Last Round`))
    (:`then_2`
      (if (`self.Is At last Round`)
        (`/Engine/EditorBlueprintResources/StandardMacros.DoOnce` false
          (:`Completed`
            (bind _returnvalue (`GameplayStatics.SpawnSound2D` "/Game/AI/RonnyBossFight/BossTheme_Cue.BossTheme_Cue" 1.0 1.0 0.0 null false false))
            (set `self.SoundCueHandle` _returnvalue)))))
    (:`then_3`
      (`self.is last round finished`))))

(event `self.RoundEnded`
  (`self.DisplaySkills`))

(event `self.GetGameManager`
  (bind _returnvalue (`GameplayStatics.GetActorOfClass` "/Game/GameManagers/BP_GameManager.BP_GameManager_C"))
  (add `/Game/GameManagers/BP_GameManager.OnNewRound` _returnvalue (delegate `OnNewRound_Event`)))

(event `OnNewRound_Event`
  (`self.OnNewRoundBegin`))

(event `Remaining enemies event`
  (set `self.Remaining Enemies` (- (`self.SpawnCount`) (`self.EnemiesKilled`)))
  (if (<= (`self.Remaining Enemies`) 3)
    (`self.ShowAI`)
    (else
      (`self.DoNotShow`))))

(event `Get Last Round`
  (if (`KismetMathLibrary.Conv_IntToBool` (+ (- (`self.CurrentRound`) (`KismetArrayLibrary.Array_LastIndex` (`self.AllRounds`))) 1))
    (set `self.Is At last Round` true)))

(event `is last round finished`
  (if (== (`KismetArrayLibrary.Array_Length` (`self.AllRounds`)) (`self.CurrentRound`))
    (set `self.Last Round Finished` true)
    (`AudioComponent.Stop` (`self.SoundCueHandle`))))

(event `ShowAI`
  (bind _outactors (`GameplayStatics.GetAllActorsOfClass` "/Game/AI/Bp_EnemyBase.Bp_EnemyBase_C"))
  (for _array_element _outactors
    (`PrimitiveComponent.SetRenderCustomDepth` (`Character.Mesh` _array_element) true)))

(event `DoNotShow`
  (bind _outactors (`GameplayStatics.GetAllActorsOfClass` "/Game/AI/Bp_EnemyBase.Bp_EnemyBase_C"))
  (for _array_element _outactors
    (`PrimitiveComponent.SetRenderCustomDepth` (`Character.Mesh` _array_element) false)))

(fn `UserConstructionScript`)