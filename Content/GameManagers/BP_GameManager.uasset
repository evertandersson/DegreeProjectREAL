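; BP_GameManager runs the between-round upgrade choice, showing skill cards and applying the player's pick.
; It creates a hidden WB_UpgradeScreen and binds to BP_EnemySpawner's AssignDisplaySkills, which triggers display of random upgrades from ACSkillUpgradeManager.
; UnlockSkill uses GAS to either grant an ability, removing it from the available pool, or apply a leveled GameplayEffect.
; It then calls OnNewRound.
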(event Custom|UnlockSkill
  (params (Skill%20index :type Integer))
  (bind _currentchoosableskills (Variables|Default|GetCurrentChoosableSkills))
  (bind _ac_skillupgrademanager (Variables|Default|GetAC_SkillUpgradeManager))
  (bind _output (Utilities|Array|Get(acopy) _currentchoosableskills Skill%20index))
  (bind _availableupgrades (Variables|/Script/DegreeProject.SkillUpgradeManager|GetAvailableUpgrades _ac_skillupgrademanager))
  (bind _returnvalue (Utilities|Array|FindItem _availableupgrades _output))
  (bind _asbp_third_person_character (Utilities|Casting|CastToBP_ThirdPersonCharacter (Game|Player|GetPlayerPawn 0)))
  (bind _returnvalue_2 (Class|SkillUpgradeManager|ApplyUpgrade (Variables|Default|GetAC_SkillUpgradeManager) _asbp_third_person_character _returnvalue))
  (if (.bIsSkillUpgrade (Utilities|Struct|BreakSkillUpgrade _returnvalue_2))
    (GameplayAbilities|GiveAbility (Variables|/Script/DegreeProject.DegreeProjectCharacter|GetAbilitySystemComponent _asbp_third_person_character) (.SkillToUnlock (Utilities|Struct|BreakSkillUpgrade _returnvalue_2)) 0 -1)
    (Utilities|Array|Add (Variables|/Game/ThirdPerson/Blueprints/BP_ThirdPersonCharacter.BP_ThirdPersonCharacter_C|GetCurrentAbilityListUsed _asbp_third_person_character) (.SkillToUnlock (Utilities|Struct|BreakSkillUpgrade _returnvalue_2)))
    (Class|SkillUpgradeManager|RemoveSkillfromAvailableUpgrades (Variables|Default|GetAC_SkillUpgradeManager) _returnvalue)
    (else
      (GameplayEffects|ApplyGameplayEffectToSelf :self (Variables|/Script/DegreeProject.DegreeProjectCharacter|GetAbilitySystemComponent _asbp_third_person_character) :GameplayEffectClass (.EffectType (Utilities|Struct|BreakSkillUpgrade _returnvalue_2)) :Level (.Level (Utilities|Struct|BreakSkillUpgrade _returnvalue_2)))))
  (Variables|Default|SetbChooseSkill false)
  (Default|CallOnNewRound))

(event Custom|DisplaySkills_Event
  (bind _outpickedskills (Class|SkillUpgradeManager|GetRandomUpgrades (Variables|Default|GetAC_SkillUpgradeManager)))
  (bind _output_get (Variables|Default|SetCurrentChoosableSkills _outpickedskills))
  (for _array_element _output_get
    (Development|PrintString (Utilities|GetClassDisplayName (.effecttype _array_element)))
    (Variables|Default|SetbChooseSkill true)
    (Default|DisplaySkills (Variables|Default|GetSkillCardsWidget) _output_get self)))

(event EventBeginPlay
  (bind _returnvalue (UserInterface|CreateWidget "/Game/HUD/WB_UpgradeScreen.WB_UpgradeScreen_C"))
  (bind _output_get (Variables|Default|SetSkillCardsWidget _returnvalue))
  (UserInterface|Viewport|AddtoViewport _output_get 0)
  (Widget|SetVisibility _output_get "Hidden")
  (bind _returnvalue_2 (Actor|GetActorOfClass "/Game/GameManagers/BP_EnemySpawner.BP_EnemySpawner_C"))
  (Utilities|IsValid _returnvalue_2
    (:Is%20Valid
      (EventDispatchers|AssignDisplaySkills _returnvalue_2 (delegate Custom|DisplaySkills_Event)))))

(event Input|KeyboardEvents|DebugKeySpaceBar
  (params (Key :type Key%20Structure :default "None") (ActionValue :type Input%20Action%20Value%20Structure)))

(fn ConstructionScript)