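; Pooled griffon enemy that uses the Gameplay Ability System for damage and shows a health bar turned toward the player camera.
; Hits apply GE_Damage through a set-by-caller magnitude, and claw sphere overlaps damage the player through the Damagable interface.
; Death plays sound and montage, then reports to BP_EnemySpawner or returns to the pool.
; Pool spawns snap to the ground by line trace; Knockback and ResetHealth are empty stubs.
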(event `self.ReceiveBeginPlay`
  (bind _aswbp_enemy_widget (cast `/Game/HUD/Enemy_HUD/WBP_EnemyWidget` (`WidgetComponent.GetWidget` (`self.Widget`))))
  (set `self.EnemyWidget` _aswbp_enemy_widget)
  (bind _returnvalue (`GameplayStatics.GetActorOfClass` "/Game/GameManagers/BP_EnemySpawner.BP_EnemySpawner_C"))
  (`/Engine/EditorBlueprintResources/StandardMacros.IsValid` _returnvalue
    (:`Is Valid`
      (set `self.EnemySpawner` _returnvalue))))

(event `self.ReceiveTick`
  (params (DeltaSeconds :type "Float (single-precision)"))
  (bind _abilitysystem2 (`self.AbilitySystem2`))
  (bind _widget (`self.Widget`))
  (`/Game/HUD/Enemy_HUD/WBP_EnemyWidget.UpdateHealthBar` (`self.EnemyWidget`) (/ (`.ReturnValue` (`AbilitySystemBlueprintLibrary.GetFloatAttributeFromAbilitySystemComponent` _abilitysystem2 (struct :`AttributeName` "CurrentHealth" :`Attribute` "/Script/DegreeProject.StandardAttributeSet:CurrentHealth" :`AttributeOwner` "/Script/CoreUObject.Class'/Script/DegreeProject.StandardAttributeSet'"))) (`.ReturnValue` (`AbilitySystemBlueprintLibrary.GetFloatAttributeFromAbilitySystemComponent` _abilitysystem2 (struct :`AttributeName` "MaxHealth" :`Attribute` "/Script/DegreeProject.StandardAttributeSet:MaxHealth" :`AttributeOwner` "/Script/CoreUObject.Class'/Script/DegreeProject.StandardAttributeSet'")))))
  (`SceneComponent.K2_SetWorldRotation` _widget (`KismetMathLibrary.FindLookAtRotation` (`SceneComponent.K2_GetComponentLocation` _widget) (`SceneComponent.K2_GetComponentLocation` (`PlayerCameraManager.TransformComponent` (`GameplayStatics.GetPlayerCameraManager` 0)))) false false))

(event `self.TakeDamage`
  (params (AbilitySystem :type "AbilitySystemComponent Object Reference"))
  (if (not (`self.IsDead`))
    (bind _returnvalue (`AbilitySystemBlueprintLibrary.AssignTagSetByCallerMagnitude` (`AbilitySystemComponent.MakeOutgoingSpec` AbilitySystem "/Game/Ablities/Combat/GE_Damage.GE_Damage_C" 2.0 (`AbilitySystemComponent.MakeEffectContext` AbilitySystem)) (struct :`TagName` "Effect.Damage") 1.0))
    (`AbilitySystemComponent.BP_ApplyGameplayEffectSpecToSelf` (`self.AbilitySystem2`) _returnvalue)
    (`self.Knockback`)))

(event `self.HandleDeath`
  (bind _enemyspawner (`self.EnemySpawner`))
  (`self.Knockback`)
  (`GameplayStatics.PlaySoundAtLocation` "/Game/QuadrapedCreatures/Griffon/BluePrints/eagleSFX.eagleSFX" (`self.K2_GetActorLocation`) (struct) 1.0 1.0 0.0 null null null null)
  (`self.ResetHealth`)
  (`self.OnAttackEnd`)
  (set `self.IsDead` true)
  (`|PlayMontage` (`self.Mesh`) "/Game/QuadrapedCreatures/Griffon/Animations/AM_GriffithDeath.AM_GriffithDeath"
    (:`OnCompleted`
      (`/Engine/EditorBlueprintResources/StandardMacros.IsValid` _enemyspawner
        (:`Is Valid`
          (`EnemySpawner.AddEnemyKilled` _enemyspawner self)
          (set `self.IsDead` false))
        (:`Is Not Valid`
          (`self.OnReturnToPool`))))))

(event `self.OnSpawnFromPool`
  (`self.SetActorHiddenInGame` false)
  (`PrimitiveComponent.SetCollisionEnabled` (`self.CapsuleComponent`) "QueryAndPhysics")
  (bind _outhit (`KismetSystemLibrary.LineTraceSingle` (`self.K2_GetActorLocation`) (+ (`self.K2_GetActorLocation`) (* (* (`self.GetActorUpVector`) -1.0) 2000.0)) "TraceTypeQuery1"))
  (`self.K2_SetActorLocation` (`KismetMathLibrary.MakeVector` (.x (`.Location` (`GameplayStatics.BreakHitResult` _outhit))) (.y (`.Location` (`GameplayStatics.BreakHitResult` _outhit))) (+ (.z (`.Location` (`GameplayStatics.BreakHitResult` _outhit))) (`CapsuleComponent.CapsuleHalfHeight` (`self.CapsuleComponent`))))))

(event `self.OnReturnToPool`
  (`self.SetActorHiddenInGame` true)
  (`PrimitiveComponent.SetCollisionEnabled` (`self.CapsuleComponent`) "NoCollision")
  (`self.K2_SetActorLocation` (10000.0 10000.0 10000.0)))

(event `/Game/ThirdPerson/Blueprints/Interfaces/I_Enemy.DealDamageToPlayer`
  (bind _returnvalue (`GameplayStatics.GetPlayerCharacter` 0))
  (bind _outactors (`KismetSystemLibrary.SphereOverlapActors` (`SceneComponent.K2_GetComponentLocation` (`self.Claws`)) 100.0 (`|MakeArray` "ObjectTypeQuery3" :!type "EObjectTypeQuery Enum") "/Game/ThirdPerson/Blueprints/BP_ThirdPersonCharacter.BP_ThirdPersonCharacter_C" (`|MakeArray` self :!type "Actor Object Reference")))
  (for _ _outactors
    (if (`KismetSystemLibrary.DoesClassImplementInterface` (`GameplayStatics.GetObjectClass` _returnvalue) "/Script/DegreeProject.Damagable")
      (message `Damagable.TakeDamage` _returnvalue (`self.AbilitySystem2`)))))

(fn `EnableCollision`
  (params (Enable :type Boolean) (CollisionModeMesh :type "ECollisionEnabled Enum" :default "NoCollision") (CollisionModeCapsule :type "ECollisionEnabled Enum" :default "NoCollision")))

(fn `GetEnemyRef`
  (returns (EnemyRef :type "/Game/AI/Bp_EnemyBase Object Reference"))
  (return null))

(fn `Knockback`)

(fn `ResetHealth`)

(fn `UserConstructionScript`)