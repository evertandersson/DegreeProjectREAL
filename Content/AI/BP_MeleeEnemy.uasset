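; Melee enemy Blueprint that damages the player with its sword through a DealDamagetoPlayer event.
; The event runs a pawn sphere overlap at the SwordCollider's location, filtered to BP_ThirdPersonCharacter.
; For each hit, it checks player 0's character for the Damagable interface and sends TakeDamageMessage with its AbilitySystem, flagged as a non-jump attack.
; BeginPlay and the construction script only call their parents.
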(event `self.ReceiveBeginPlay`
  (`parent.ReceiveBeginPlay`))

(event `self.DealDamageToPlayer`
  (bind _returnvalue (`GameplayStatics.GetPlayerCharacter` 0))
  (bind _outactors (`KismetSystemLibrary.SphereOverlapActors` (`SceneComponent.K2_GetComponentLocation` (`self.SwordCollider`)) 50.0 (`|MakeArray` "ObjectTypeQuery3" :!type "EObjectTypeQuery Enum") "/Game/ThirdPerson/Blueprints/BP_ThirdPersonCharacter.BP_ThirdPersonCharacter_C" (`|MakeArray` self :!type "Actor Object Reference")))
  (for _ _outactors
    (if (`KismetSystemLibrary.DoesClassImplementInterface` (`GameplayStatics.GetObjectClass` _returnvalue) "/Script/DegreeProject.Damagable")
      (message `Damagable.TakeDamage` _returnvalue (`self.AbilitySystem`) false))))

(fn `UserConstructionScript`
  (`parent.UserConstructionScript`))