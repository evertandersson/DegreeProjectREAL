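; BP_NPC is a pooled enemy NPC that caches the player character and the enemy spawner on BeginPlay.
; Spawning from the pool unhides it, enables capsule collision and traces downward to stand it on the surface below.
; Returning to the pool hides it, disables collision and moves it to a distant holding location.
; Logic reporting a kill to the spawner on player contact is disconnected, leaving the hit event empty.
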(event `self.ReceiveBeginPlay`
  (bind _asbp_third_person_character (cast `/Game/ThirdPerson/Blueprints/BP_ThirdPersonCharacter` (`GameplayStatics.GetPlayerPawn` 0)))
  (set `self.Player` _asbp_third_person_character)
  (bind _returnvalue (`GameplayStatics.GetActorOfClass` "/Game/GameManagers/BP_EnemySpawner.BP_EnemySpawner_C"))
  (set `self.EnemySpawner` _returnvalue))

(event `self.CapsuleComponent.OnComponentHit`
  (params (HitComponent :type "PrimitiveComponent Object Reference") (OtherActor :type "Actor Object Reference") (OtherComp :type "PrimitiveComponent Object Reference") (NormalImpulse :type "Vector Structure") (Hit :type "HitResult Structure (by ref)")))

(event `self.OnSpawnFromPool`
  (`self.SetActorHiddenInGame` false)
  (`PrimitiveComponent.SetCollisionEnabled` (`self.CapsuleComponent`) "QueryAndPhysics")
  (bind _outhit (`KismetSystemLibrary.LineTraceSingle` (`self.K2_GetActorLocation`) (+ (`self.K2_GetActorLocation`) (* (* (`self.GetActorUpVector`) -1.0) 2000.0)) "TraceTypeQuery1"))
  (`self.K2_SetActorLocation` (`KismetMathLibrary.MakeVector` (.x (`.Location` (`GameplayStatics.BreakHitResult` _outhit))) (.y (`.Location` (`GameplayStatics.BreakHitResult` _outhit))) (+ (.z (`.Location` (`GameplayStatics.BreakHitResult` _outhit))) (`CapsuleComponent.CapsuleHalfHeight` (`self.CapsuleComponent`))))))

(event `self.OnReturnToPool`
  (`self.SetActorHiddenInGame` true)
  (`PrimitiveComponent.SetCollisionEnabled` (`self.CapsuleComponent`) "NoCollision")
  (`self.K2_SetActorLocation` (10000.0 10000.0 10000.0)))

(fn `UserConstructionScript`)