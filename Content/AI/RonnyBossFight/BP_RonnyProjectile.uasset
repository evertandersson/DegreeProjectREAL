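; Pooled projectile for the Ronny boss fight that flies forward by a fixed step each tick, independent of delta time.
; The first sphere overlap with a GAS owner passes the supplied ability system in a damage message and spawns a water-ball hit effect.
; After a short delay it returns to the pool, which hides it and moves it far away; respawning unhides it and clears the hit flag.
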(event `self.Sphere.OnComponentBeginOverlap`
  (params (OverlappedComponent :type "PrimitiveComponent Object Reference") (OtherActor :type "Actor Object Reference") (OtherComp :type "PrimitiveComponent Object Reference") (OtherBodyIndex :type Integer) (bFromSweep :type Boolean) (SweepResult :type "HitResult Structure (by ref)"))
  (bind _abilitysystem (`self.AbilitySystem`))
  (if (and (`KismetSystemLibrary.DoesImplementInterface` OtherActor "/Game/ThirdPerson/Blueprints/Interfaces/I_GASOwner.I_GASOwner_C") (not (`self.HasHit`)))
    (`/Engine/EditorBlueprintResources/StandardMacros.IsValid` _abilitysystem
      (:`Is Valid`
        (set `self.HasHit` true)
        (message `Damagable.TakeDamage` OtherActor _abilitysystem)
        (`GameplayStatics.SpawnEmitterAtLocation` "/Game/FXVarietyPack/Particles/P_ky_waterBallHit.P_ky_waterBallHit" (`self.K2_GetActorLocation`) (struct) (1.0 1.0 1.0) true "AutoRelease")
        (`KismetSystemLibrary.Delay` 0.1)
        (`Poolable.OnReturnToPool`)))))

(event `self.ReceiveTick`
  (params (DeltaSeconds :type "Float (single-precision)"))
  (`self.K2_SetActorLocation` (+ (`self.K2_GetActorLocation`) (* (`self.GetActorForwardVector`) 25.0))))

(event `/Game/AI/RonnyBossFight/I_GetAbilitySystem.SetAbilitySystem`
  (params (AbilitySystem :type "AbilitySystemComponent Object Reference"))
  (set `self.AbilitySystem` AbilitySystem))

(event `self.OnSpawnFromPool`
  (`self.SetActorHiddenInGame` false)
  (set `self.HasHit` false))

(event `self.OnReturnToPool`
  (`self.SetActorHiddenInGame` true)
  (`self.K2_SetActorLocation` (10000.0 10000.0 10000.0)))

(fn `UserConstructionScript`)