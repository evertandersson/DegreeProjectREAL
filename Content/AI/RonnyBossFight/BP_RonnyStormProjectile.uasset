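; Pooled storm projectile for the Ronny boss fight that chases the player and tosses them upward.
; A timeline scales it up on spawn and reverses after its lifespan to return it to the pool.
; Each tick, an outer capsule drags characters inward by distance-scaled offsets, while an inner capsule launches them up.
; Exiting above the inner capsule deals damage through the passed ability system and blocks further captures.
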(event `self.OnSpawnFromPool`
  ; Handle Pooling
  (set `self.HasHit` false)
  (`self.SetActorScale3D` (0.2 0.2 0.2))
  (`self.SetActorHiddenInGame` false)
  (`self.Resize` true)
  (`KismetSystemLibrary.Delay` (`self.LifeSpan`))
  (if (`KismetArrayLibrary.Array_Contains` (`self.AffectedActorsPull`) (`GameplayStatics.GetPlayerPawn` 0))
    (set `self.DestroyWhenEmpty` true)
    (else
      (`self.Resize` false))))

(event `self.OnReturnToPool`
  ; Handle Pooling
  (`self.SetActorHiddenInGame` false)
  (`self.K2_SetActorLocation` (10000.0 10000.0 10000.0)))

(event `Resize`
  (params (ScaleUp :type Boolean))
  (if ScaleUp
    (bind (_direction _size) (`Timeline|Timeline` :!via `PlayFromStart` :!label _label)
      (:`Update`
        (`self.SetActorScale3D` (`KismetMathLibrary.Conv_DoubleToVector` _size)))
      (:`Finished`
        (if (not ScaleUp)
          (message `IHasGroundPos.IsInStorm` (`GameplayStatics.GetPlayerPawn` 0) false)
          (`Poolable.OnReturnToPool`))))
    (else
      (goto _label :!via `ReverseFromEnd`))))

(event `self.ReceiveTick`
  (params (DeltaSeconds :type "Float (single-precision)"))
  (bind _returnvalue (`GameplayStatics.GetPlayerPawn` 0))
  (`|ExecutionSequence`
    (:`then_0`
      (if (`self.DestroyWhenEmpty`)
        (`/Engine/EditorBlueprintResources/StandardMacros.DoOnce` false
          (:`Completed`
            (`self.Resize` false)))))
    (:`then_1`
      (`|AIMoveTo` self (`self.K2_GetActorLocation` _returnvalue) _returnvalue))
    (:`then_2`
      ;[0.15 0.15 0.15 0.5 25] Launch Character towards storm
      (for _array_element (`self.AffectedActorsPull`)
        (if (`GameplayStatics.ObjectIsA` _array_element "/Game/ThirdPerson/Blueprints/BP_ThirdPersonCharacter.BP_ThirdPersonCharacter_C")
          (bind _returnvalue_2 (- (`self.K2_GetActorLocation`) (`self.K2_GetActorLocation` _array_element)))
          (`self.K2_AddActorWorldOffset` _array_element (`KismetMathLibrary.MakeVector` (.x (* (* (`KismetMathLibrary.Normal` _returnvalue_2) (/ (`self.PullStrength`) (`KismetMathLibrary.MapRangeClamped` (`KismetMathLibrary.VSize` _returnvalue_2) 0.0 (* (`CapsuleComponent.CapsuleRadius` (`self.CapsulePullForce`)) 2.0) 0.0 10.0))) (`GameplayStatics.GetWorldDeltaSeconds`))) (.y (* (* (`KismetMathLibrary.Normal` _returnvalue_2) (/ (`self.PullStrength`) (`KismetMathLibrary.MapRangeClamped` (`KismetMathLibrary.VSize` _returnvalue_2) 0.0 (* (`CapsuleComponent.CapsuleRadius` (`self.CapsulePullForce`)) 2.0) 0.0 10.0))) (`GameplayStatics.GetWorldDeltaSeconds`)))) false false))))
    (:`then_3`
      ;[0.15 0.15 0.15 0.5 25] Launch Character Up when close enough
      (for _array_element_2 (`self.AffectedActorsUpForce`)
        (if (`GameplayStatics.ObjectIsA` _array_element_2 "/Game/ThirdPerson/Blueprints/BP_ThirdPersonCharacter.BP_ThirdPersonCharacter_C")
          (message `IHasGroundPos.LaunchCharacterInDirection` _array_element_2 (`KismetMathLibrary.MakeVector` 0.0 0.0 (`KismetMathLibrary.MapRangeClamped` (+ (.z (`KismetMathLibrary.Vector_GetAbs` (- (`self.K2_GetActorLocation` _array_element_2) (`self.K2_GetActorLocation`)))) 1.0) 0.0 600.0 20.0 50.0)) true))))))

(event `self.CapsulePullForce.OnComponentBeginOverlap`
  (params (OverlappedComponent :type "PrimitiveComponent Object Reference") (OtherActor :type "Actor Object Reference") (OtherComp :type "PrimitiveComponent Object Reference") (OtherBodyIndex :type Integer) (bFromSweep :type Boolean) (SweepResult :type "HitResult Structure (by ref)"))
  ; Handle Overlap pull force
  (if (not (`self.HasHit`))
    (`KismetArrayLibrary.Array_Add` (`self.AffectedActorsPull`) OtherActor)))

(event `self.CapsulePullForce.OnComponentEndOverlap`
  (params (OverlappedComponent :type "PrimitiveComponent Object Reference") (OtherActor :type "Actor Object Reference") (OtherComp :type "PrimitiveComponent Object Reference") (OtherBodyIndex :type Integer))
  ; Handle Overlap pull force
  (`KismetArrayLibrary.Array_RemoveItem` (`self.AffectedActorsPull`) OtherActor))

(event `self.CapsuleUpForce.OnComponentBeginOverlap`
  (params (OverlappedComponent :type "PrimitiveComponent Object Reference") (OtherActor :type "Actor Object Reference") (OtherComp :type "PrimitiveComponent Object Reference") (OtherBodyIndex :type Integer) (bFromSweep :type Boolean) (SweepResult :type "HitResult Structure (by ref)"))
  ; Handle overlap actors up force
  (if (and (`KismetSystemLibrary.DoesClassImplementInterface` (`GameplayStatics.GetObjectClass` OtherActor) "/Script/DegreeProject.IHasGroundPos") (not (`self.HasHit`)))
    (`KismetArrayLibrary.Array_Add` (`self.AffectedActorsUpForce`) OtherActor)
    (message `IHasGroundPos.IsInStorm` OtherActor true)))

(event `self.CapsuleUpForce.OnComponentEndOverlap`
  (params (OverlappedComponent :type "PrimitiveComponent Object Reference") (OtherActor :type "Actor Object Reference") (OtherComp :type "PrimitiveComponent Object Reference") (OtherBodyIndex :type Integer))
  (bind (_returnvalue_x _returnvalue_y _returnvalue_z) (`KismetMathLibrary.BreakVector` (`self.K2_GetActorLocation` OtherActor)))
  (bind (_returnvalue_x_2 _returnvalue_y_2 _returnvalue_z_2) (`KismetMathLibrary.BreakVector` (`self.K2_GetActorLocation`)))
  ; Handle overlap actors up force
  (if (and (`GameplayStatics.ObjectIsA` OtherActor "/Game/ThirdPerson/Blueprints/BP_ThirdPersonCharacter.BP_ThirdPersonCharacter_C") (not (`self.HasHit`)) (> _returnvalue_z (+ _returnvalue_z_2 (`CapsuleComponent.CapsuleHalfHeight` (`self.CapsuleUpForce`)))))
    (message `Damagable.TakeDamage` OtherActor (`self.Ability System`))
    (message `IHasGroundPos.IsInStorm` OtherActor false)
    (set `self.HasHit` true))
  (`KismetArrayLibrary.Array_RemoveItem` (`self.AffectedActorsUpForce`) OtherActor))

(event `/Game/AI/RonnyBossFight/I_GetAbilitySystem.SetAbilitySystem`
  (params (AbilitySystem :type "AbilitySystemComponent Object Reference"))
  (set `self.Ability System` AbilitySystem))

(fn `UserConstructionScript`)