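; Ronny boss enemy character with ranged, storm and explosion attacks, plus a knockback away from the player.
; Attacks spawn pooled projectiles from the pelvis, at a downward trace hit or attached to the back socket.
; Each projectile receives the boss's Ability System, and each attack signals its end after a delay.
; Tick updates the health bar from ability attributes and turns the HUD toward the camera.
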(event `self.Attack`
  (bind _returnvalue (`self.K2_GetActorLocation`))
  ;[0.15 0.15 0.15 0.5 30] Ranged Attack
  (`GameplayStatics.PlaySoundAtLocation` "/Game/SFX/RonnySoundEffects/cough-and-spit-40131_Cue.cough-and-spit-40131_Cue" _returnvalue (struct) 1.0 1.0 0.0 null null null null)
  (`KismetSystemLibrary.MoveComponentTo` (`self.CapsuleComponent`) _returnvalue (`KismetMathLibrary.MakeRotator` (.roll (`KismetMathLibrary.MakeRotFromX` (`KismetMathLibrary.Normal` (- (`self.K2_GetActorLocation` (`GameplayStatics.GetPlayerPawn` 0)) _returnvalue)))) 0.0 (.yaw (`KismetMathLibrary.MakeRotFromX` (`KismetMathLibrary.Normal` (- (`self.K2_GetActorLocation` (`GameplayStatics.GetPlayerPawn` 0)) _returnvalue))))) false false 2.0)
  (`self.LaunchCharacter` (+ (* (`self.GetActorUpVector`) 200.0) (* (* (`self.GetActorForwardVector`) -1.0) 200.0)))
  (bind _spawnedactor (`PoolSubsystem.SpawnFromPool` :`self` (subsystem `PoolSubsystem`) :`PoolClass` "/Game/AI/RonnyBossFight/BP_RonnyProjectile.BP_RonnyProjectile_C" :`Location` (`KismetMathLibrary.MakeVector` (.x (.location (`SkinnedMeshComponent.GetBoneTransform` (`self.Mesh`) "Pelvis" "RTS_World"))) (.y (.location (`SkinnedMeshComponent.GetBoneTransform` (`self.Mesh`) "Pelvis" "RTS_World"))) (+ (.z (.location (`SkinnedMeshComponent.GetBoneTransform` (`self.Mesh`) "Pelvis" "RTS_World"))) 70.0))))
  (set `MovementComponent.Velocity` (* (`KismetMathLibrary.Conv_RotatorToVector` (.rotation (`SkinnedMeshComponent.GetBoneTransform` (`self.Mesh`) "Pelvis" "RTS_World"))) 5000.0) (`/Game/AI/RonnyBossFight/BP_RonnyProjectile.ProjectileMovement` _spawnedactor))
  (message `/Game/AI/RonnyBossFight/I_GetAbilitySystem.SetAbilitySystem` _spawnedactor (`self.AbilitySystem`))
  (`KismetSystemLibrary.Delay` 1.0)
  (`self.OnAttackEnd`))

(event `StormAttack`
  (bind _returnvalue (`self.K2_GetActorLocation`))
  ;[0.15 0.15 0.15 0.5 30] Storm Attack
  (bind _outhit (`KismetSystemLibrary.LineTraceSingle` :`Start` _returnvalue :`End` (+ _returnvalue (* (`self.GetActorUpVector`) -200.0)) :`TraceChannel` "TraceTypeQuery1" :`DrawDebugType` "ForDuration"))
  (bind _spawnedactor (`PoolSubsystem.SpawnFromPool` :`self` (subsystem `PoolSubsystem`) :`PoolClass` "/Game/AI/RonnyBossFight/BP_RonnyStormProjectile.BP_RonnyStormProjectile_C" :`Location` (`KismetMathLibrary.MakeVector` (.x (`.Location` (`GameplayStatics.BreakHitResult` _outhit))) (.y (`.Location` (`GameplayStatics.BreakHitResult` _outhit))) (+ (.z (`.Location` (`GameplayStatics.BreakHitResult` _outhit))) 100.0))))
  (message `/Game/AI/RonnyBossFight/I_GetAbilitySystem.SetAbilitySystem` _spawnedactor (`self.AbilitySystem`))
  (`KismetSystemLibrary.Delay` 1.0)
  (`self.OnAttackEnd`))

(event `Explosion Attack`
  (bind _spawnedactor (`PoolSubsystem.SpawnFromPool` (subsystem `PoolSubsystem`) "/Game/AI/RonnyBossFight/BP_ExplosionProjectile.BP_ExplosionProjectile_C" (.location (`SkinnedMeshComponent.GetBoneTransform` (`self.Mesh`) "Pelvis" "RTS_World")) (.rotation (`SkinnedMeshComponent.GetBoneTransform` (`self.Mesh`) "Pelvis" "RTS_World"))))
  (`self.K2_AttachToComponent` _spawnedactor (`self.Mesh`) "backSocket" "KeepWorld" "KeepWorld" "KeepWorld" true)
  (message `/Game/AI/RonnyBossFight/I_GetAbilitySystem.SetAbilitySystem` _spawnedactor (`self.AbilitySystem`))
  (`KismetSystemLibrary.Delay` 5.0)
  (`self.OnAttackEnd`))

(event `self.ReceiveTick`
  (params (DeltaSeconds :type "Float (single-precision)"))
  (bind _abilitysystem (`self.AbilitySystem`))
  (bind _hud (`self.HUD`))
  (`/Game/HUD/Enemy_HUD/WBP_EnemyWidget.UpdateHealthBar` (`self.Enemy Health Widget`) (/ (`.ReturnValue` (`AbilitySystemBlueprintLibrary.GetFloatAttributeFromAbilitySystemComponent` _abilitysystem (struct :`AttributeName` "CurrentHealth" :`Attribute` "/Script/DegreeProject.StandardAttributeSet:CurrentHealth" :`AttributeOwner` "/Script/CoreUObject.Class'/Script/DegreeProject.StandardAttributeSet'"))) (`.ReturnValue` (`AbilitySystemBlueprintLibrary.GetFloatAttributeFromAbilitySystemComponent` _abilitysystem (struct :`AttributeName` "MaxHealth" :`Attribute` "/Script/DegreeProject.StandardAttributeSet:MaxHealth" :`AttributeOwner` "/Script/CoreUObject.Class'/Script/DegreeProject.StandardAttributeSet'")))))
  (`SceneComponent.K2_SetWorldRotation` _hud (`KismetMathLibrary.FindLookAtRotation` (`SceneComponent.K2_GetComponentLocation` _hud) (`SceneComponent.K2_GetComponentLocation` (`PlayerCameraManager.TransformComponent` (`GameplayStatics.GetPlayerCameraManager` 0)))) false false))

(fn `Knockback`
  (`self.LaunchCharacter` (`KismetMathLibrary.MakeVector` (.x (* (`KismetMathLibrary.Normal` (- (`self.K2_GetActorLocation`) (`self.K2_GetActorLocation` (`GameplayStatics.GetPlayerCharacter` 0)))) 1000.0)) (.y (* (`KismetMathLibrary.Normal` (- (`self.K2_GetActorLocation`) (`self.K2_GetActorLocation` (`GameplayStatics.GetPlayerCharacter` 0)))) 1000.0)) (+ (.z (* (`KismetMathLibrary.Normal` (- (`self.K2_GetActorLocation`) (`self.K2_GetActorLocation` (`GameplayStatics.GetPlayerCharacter` 0)))) 1000.0)) 100.0)) true))

(fn `UserConstructionScript`)