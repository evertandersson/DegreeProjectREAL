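; Pooled explosion projectile for the Ronny boss fight that detonates after a short delay once spawned.
; A sphere overlap tracks Damagable actors other than the boss, playing a charge sound as each enters.
; Detonation activates the particle, then damages tracked actors using the supplied ability system and launches them away from the center.
; It then returns to the pool, hidden and parked far away, avoiding respawning.
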(event `self.OnSpawnFromPool`
  ; Handle object pooling
  (`self.SetActorHiddenInGame` false)
  (`KismetSystemLibrary.Delay` 2.0)
  (`ActorComponent.Activate` (`self.ExplosionParticle`) false)
  (`self.ExplodeActors`))

(event `self.OnReturnToPool`
  ; Handle object pooling
  (`self.SetActorHiddenInGame` true)
  (`self.K2_SetActorLocation` (10000.0 10000.0 10000.0)))

(event `ExplodeActors`
  (for _array_element (`self.AffectedActors`)
    (`/Engine/EditorBlueprintResources/StandardMacros.IsValid` _array_element
      (:`Is Valid`
        (message `Damagable.TakeDamage` _array_element (`self.AbilitySystem`) false)
        (`/Engine/EditorBlueprintResources/StandardMacros.IsValid` _array_element
          (:`Is Valid`
            (bind _returnvalue (`self.K2_GetActorLocation` _array_element))
            (`GameplayStatics.PlaySoundAtLocation` "/Game/StarterContent/Audio/Explosion_Cue.Explosion_Cue" _returnvalue (struct) 1.0 1.0 0.0 null null null null)
            (message `IHasGroundPos.LaunchCharacterInDirection` _array_element (* (`KismetMathLibrary.Normal` (- _returnvalue (`self.K2_GetActorLocation`))) 3000.0) false))))))
  (`KismetSystemLibrary.Delay` 0.5)
  (`Poolable.OnReturnToPool`))

(event `self.Sphere.OnComponentBeginOverlap`
  (params (OverlappedComponent :type "PrimitiveComponent Object Reference") (OtherActor :type "Actor Object Reference") (OtherComp :type "PrimitiveComponent Object Reference") (OtherBodyIndex :type Integer) (bFromSweep :type Boolean) (SweepResult :type "HitResult Structure (by ref)"))
  (bind _isplayer (`self.ImplementsInterface` OtherActor))
  (if _isplayer
    (`KismetArrayLibrary.Array_Add` (`self.AffectedActors`) OtherActor)
    (`GameplayStatics.PlaySoundAtLocation` "/Game/SFX/RonnySoundEffects/power-charge-6798_Cue.power-charge-6798_Cue" (`self.K2_GetActorLocation`) (struct) 1.0 1.0 18.0 null null null null)))

(event `self.Sphere.OnComponentEndOverlap`
  (params (OverlappedComponent :type "PrimitiveComponent Object Reference") (OtherActor :type "Actor Object Reference") (OtherComp :type "PrimitiveComponent Object Reference") (OtherBodyIndex :type Integer))
  (bind _isplayer (`self.ImplementsInterface` OtherActor))
  (if _isplayer
    (`KismetArrayLibrary.Array_RemoveItem` (`self.AffectedActors`) OtherActor)))

(event `/Game/AI/RonnyBossFight/I_GetAbilitySystem.SetAbilitySystem`
  (params (AbilitySystem :type "AbilitySystemComponent Object Reference"))
  (set `self.AbilitySystem` AbilitySystem))

(fn `ImplementsInterface`
  (params (Actor :type "Actor Object Reference"))
  (returns (IsPlayer :type Boolean))
  (return (and (`KismetSystemLibrary.DoesImplementInterface` Actor "/Script/DegreeProject.Damagable") (not (`GameplayStatics.ObjectIsA` Actor "/Game/AI/RonnyBossFight/BP_RonnyBoss.BP_RonnyBoss_C")))))

(fn `UserConstructionScript`)