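; Player controller Blueprint that owns the on-screen HUD for health, stamina and mana.
; On BeginPlay it creates the HealthBarWidget, keeps a reference to it and adds it to the viewport.
; Three update events take current and max values, turn each into a percentage and a "current / max" text, then pass both to the matching bar on the widget.
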(event `self.ReceiveBeginPlay`
  (bind _returnvalue (`|CreateWidget` "/Game/HUD/HealthBarWidget.HealthBarWidget_C"))
  (bind _output_get (set `self.HealthBarWidgetRef` _returnvalue))
  (`UserWidget.AddToViewport` _output_get 0))

(event `/Game/HUD/BPI_HealthInterface.UpdateHealthDisplay`
  (params (CurrentHealth :type "Float (double-precision)") (MaxHealth :type "Float (double-precision)"))
  (`/Game/HUD/HealthBarWidget.UpdateHealthBar` (`self.HealthBarWidgetRef`) (/ CurrentHealth MaxHealth) (`|FormatText` "{0} / {1}" CurrentHealth MaxHealth)))

(event `/Game/HUD/BPI_HealthInterface.UpdateStaminaDisplay`
  (params (CurrentStamina :type "Float (double-precision)") (MaxStamina :type "Float (double-precision)"))
  (`/Game/HUD/HealthBarWidget.UpdateStaminaBar` (`self.HealthBarWidgetRef`) (`|FormatText` "{0} / {1}" CurrentStamina MaxStamina) (/ CurrentStamina MaxStamina)))

(event `/Game/HUD/BPI_HealthInterface.UpdateManaDisplay`
  (params (CurrentMana :type "Float (double-precision)") (MaxMana :type "Float (double-precision)"))
  (`/Game/HUD/HealthBarWidget.UpdateManaBar` (`self.HealthBarWidgetRef`) (`|FormatText` "{0} / {1}" CurrentMana MaxMana) (/ CurrentMana MaxMana)))

(fn `UserConstructionScript`)